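; BP_Spawn is a spawn point actor that registers itself as the player's spawn when BP_Player overlaps it.
; On overlap it passes itself to the player's SetSpawn and switches its Cylinder to the active material.
; Reset restores the inactive material, and SpawnInitialise applies the active look without registering the spawn, leaving both events to be triggered externally.
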(event Custom|Reset
  (Rendering|Material|SetMaterial (Variables|Default|GetCylinder) 0 "/Game/PlayerBPs/SpawnMat.SpawnMat"))

(event Custom|SpawnInitialise
  (Rendering|Material|SetMaterial (Variables|Default|GetCylinder) 0 "/Game/PlayerBPs/ActiveSpawnMat.ActiveSpawnMat"))

(event EventBeginPlay)

(event EventTick
  (params (DeltaSeconds :type Float%20%28single-precision%29)))

(event Collision|EventActorBeginOverlap
  (params (OtherActor :type Actor%20Object%20Reference))
  (bind _asbp_player (Utilities|Casting|CastToBP_Player OtherActor))
  (Default|SetSpawn _asbp_player self)
  (Rendering|Material|SetMaterial (Variables|Default|GetCylinder) 0 "/Game/PlayerBPs/ActiveSpawnMat.ActiveSpawnMat"))

(fn ConstructionScript)