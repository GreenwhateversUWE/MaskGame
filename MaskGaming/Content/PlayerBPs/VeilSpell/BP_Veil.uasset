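; BP_Veil is the veil spell actor, a timed effect shown at a given position.
; Activate moves the capsule to that position, shows the sphere, enables actor tick and starts the NSBasic12 effect.
; A timer set to the passed VeilTime calls Deactivate, which hides the sphere, disables tick and stops the effect, leaving the actor in place for reuse.
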(event Custom|Activate
  (params (VeilTime :type Float%20%28double-precision%29) (Position :type Vector))
  (Rendering|SetVisibility (Variables|Default|GetSphere) true false)
  (Actor|Tick|SetActorTickEnabled true)
  (Transformation|SetWorldLocation (Variables|Default|GetCapsule) Position false false)
  (Components|Activation|Activate (Variables|Default|GetNS_Basic_12) true)
  (Utilities|Time|SetTimerbyEvent (delegate Custom|Deactivate) VeilTime))

(event Custom|Deactivate
  (Rendering|SetVisibility (Variables|Default|GetSphere) false false)
  (Actor|Tick|SetActorTickEnabled false)
  (Components|Activation|Deactivate (Variables|Default|GetNS_Basic_12)))

(event EventBeginPlay)

(event Collision|EventActorBeginOverlap
  (params (OtherActor :type Actor%20Object%20Reference)))

(event EventTick
  (params (DeltaSeconds :type Float%20%28single-precision%29)))

(fn ConstructionScript)