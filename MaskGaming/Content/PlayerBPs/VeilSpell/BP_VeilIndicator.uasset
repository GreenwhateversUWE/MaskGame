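; BP_VeilIndicator is the targeting indicator for the player's Veil spell, previewing where the veil will appear.
; On BeginPlay it spawns a BP_Veil actor and keeps it deactivated for reuse.
; Activate shows the indicator and plays a wind-up sound, while UpdateLocation teleports it to a given location.
; CastVeil activates that veil at the indicator's position for a fixed duration, then hides the indicator.
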(event Custom|Activate
  (Rendering|SetVisibility (Variables|Default|GetIndicator) true false)
  (Actor|Tick|SetActorTickEnabled true)
  (Audio|PlaySound2D "/Game/Sounds/WindUpSpell.WindUpSpell" 1.0 1.0 0.0 0 0))

(event Custom|Deactivate
  (Rendering|SetVisibility (Variables|Default|GetIndicator) false false)
  (Actor|Tick|SetActorTickEnabled false))

(event Custom|UpdateLocation
  (params (Location :type Vector))
  (Transformation|SetWorldLocation (Variables|Default|GetIndicator) Location false true))

(event Custom|CastVeil
  (Default|Activate (Variables|Default|GetVeilRef) 1e+01 (Transformation|GetWorldLocation (Variables|Default|GetIndicator)))
  (CallFunction|Deactivate))

(event EventBeginPlay
  (bind _returnvalue (Game|SpawnActorfromClass "/Game/PlayerBPs/VeilSpell/BP_Veil.BP_Veil_C" (Math|Transform|MakeTransform "0, 0, 0" "0, 0, 0" "1.000000,1.000000,1.000000") "Undefined" "MultiplyWithRoot" 0 0))
  (bind _output_get (Variables|Default|SetVeilRef _returnvalue))
  (Default|Deactivate _output_get))

(event Collision|EventActorBeginOverlap
  (params (OtherActor :type Actor%20Object%20Reference)))

(event EventTick
  (params (DeltaSeconds :type Float%20%28single-precision%29)))

(fn ConstructionScript)