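; Puzzle wall actor that moves toward a configurable final position, driven by an InterpToMovement component.
; BeginPlay adds FinalPosition as a control point relative to the wall's start.
; The Activation event activates the movement component, so no Tick or overlap logic is used.
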(event EventBeginPlay
  (Class|InterptoMovementComponent|AddControlPointPosition (Variables|Default|GetInterpToMovement) (Variables|Default|Getfinal%20position) true)
  (|CallParentFunction))

(event Collision|EventActorBeginOverlap
  (params (OtherActor :type Actor%20Object%20Reference))
  (|CallParentFunction OtherActor) ; This node is disabled and will not be called.\nDrag off pins to build functionality.
)

(event EventTick
  (params (DeltaSeconds :type Float%20%28single-precision%29))
  (|CallParentFunction DeltaSeconds) ; This node is disabled and will not be called.\nDrag off pins to build functionality.
)

(event EventActivation
  (Components|Activation|Activate (Variables|Default|GetInterpToMovement) false))

(fn ConstructionScript
  (|CallParentFunction))