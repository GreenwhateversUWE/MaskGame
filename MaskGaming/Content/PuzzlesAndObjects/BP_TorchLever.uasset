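; BP_TorchLever is a one-shot interactable lever, named as a torch lever, that activates linked puzzle objects.
; The first Interact calls Activation on every entry in ActivatingObjects, sets Activated to block reuse, then runs TurnLever.
; TurnLever uses a timeline to tip the mesh a quarter turn on roll or pitch, chosen from its world yaw at BeginPlay, while zeroing the other rotation axes.
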(event Custom|TurnLever
  (bind _staticmesh (Variables|Default|GetStaticMesh))
  (bind _torchfloat (Timeline|Timeline PlayFromStart)
    (:Update
      (if (Variables|Default|GetIsXAxis)
        (Transformation|SetRelativeRotation _staticmesh (Math|Rotator|MakeRotator (Math|Float|Lerp 0.0 9e+01 _torchfloat) 0.0 0.0) false false)
        (else
          (Transformation|SetRelativeRotation _staticmesh (Math|Rotator|MakeRotator 0.0 (Math|Float|Lerp 0.0 9e+01 _torchfloat) 0.0) false false))))))

(event EventBeginPlay
  (bind _staticmesh (Variables|Default|GetStaticMesh))
  (bind _returnvalue (Transformation|GetWorldRotation _staticmesh))
  (Variables|Default|SetIsXAxis (or (== (.yaw _returnvalue) 0.0) (== (.yaw _returnvalue) 1.8e+02))))

(event Collision|EventActorBeginOverlap
  (params (OtherActor :type Actor%20Object%20Reference)))

(event EventTick
  (params (DeltaSeconds :type Float%20%28single-precision%29)))

(fn ConstructionScript)

(fn Interact
  (if (not (Variables|Default|GetActivated))
    (for _array_element (Variables|Default|GetActivatingObjects)
      (Default|Activation _array_element))
    (Variables|Default|SetActivated true)
    (CallFunction|TurnLever)
    (return false)))