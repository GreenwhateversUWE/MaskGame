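; BP_Trigger is a one-shot trigger actor that switches on a referenced Whisper the first time the player enters it.
; On BeginPlay it disables the Whisper, if one is valid.
; When player character 0 begins overlapping the actor, a DoOnce gate lets a single call through to re-enable the Whisper, so later overlaps do nothing.
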(event EventBeginPlay
  (bind _whisper (Variables|Default|GetWhisper))
  (Utilities|IsValid _whisper
    (:Is%20Valid
      (Default|Enabled _whisper false))))

(event EventTick
  (params (DeltaSeconds :type Float%20%28single-precision%29)))

(event Collision|EventActorBeginOverlap
  (params (OtherActor :type Actor%20Object%20Reference))
  (bind _whisper (Variables|Default|GetWhisper))
  (if (== OtherActor (Game|GetPlayerCharacter 0))
    (Utilities|FlowControl|DoOnce false
      (:Completed
        (Utilities|IsValid _whisper
          (:Is%20Valid
            (Default|Enabled _whisper true)))))))

(fn ConstructionScript)