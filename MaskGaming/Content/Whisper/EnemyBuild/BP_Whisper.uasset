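; BP_Whisper is the Whisper enemy character, with events for enabling, knockback and movement speed.
; Enabled toggles the CharacterMovement component, while the mesh is set visible in both branches.
; Pushed stops movement, applies a velocity-change impulse with a fixed upward lift and plays one of two random damage montages.
; IsRunning and the StartSprinting/StopSprinting functions each switch max walk speed between walk and run values.
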(event Custom|Pushed
  (params (Force :type Vector))
  (bind _returnvalue (+ Force "0.000000,0.000000,100.000000"))
  (Components|Movement|StopMovementImmediately (Variables|Character|GetCharacterMovement))
  (Physics|AddImpulse (Variables|Character|GetCharacterMovement) (Math|Vector|MakeVector (.x _returnvalue) (.y _returnvalue) 1e+02) true)
  (if (> (Math|Random|RandomInteger 2) 0)
    (Animation|PlayAnimMontage "/Game/Whisper/Animations/Anim_Whisper_Taking_Damage1_Montage.Anim_Whisper_Taking_Damage1_Montage" 1.0 "None")
    (else
      (Animation|PlayAnimMontage "/Game/Whisper/Animations/Anim_Whisper_Taking_Damage2_Montage.Anim_Whisper_Taking_Damage2_Montage" 1.0 "None"))))

(event Custom|Enabled
  (params (IsEnabled :type Boolean))
  (bind _mesh (Variables|Character|GetMesh))
  (bind _charactermovement (Variables|Character|GetCharacterMovement))
  (if IsEnabled
    (Rendering|SetVisibility _mesh true false)
    (Components|Activation|SetActive _charactermovement true false)
    (else
      (Rendering|SetVisibility _mesh true false)
      (Components|Activation|SetActive _charactermovement false false))))

(event EventIsRunning
  (params (IsRunning :type Boolean))
  (if IsRunning
    (Variables|/Script/Engine.CharacterMovementComponent|SetMaxWalkSpeed (Variables|Character|GetCharacterMovement) 7e+02)
    (else
      (Variables|/Script/Engine.CharacterMovementComponent|SetMaxWalkSpeed (Variables|Character|GetCharacterMovement) 3e+02))))

(event Collision|EventActorBeginOverlap
  (params (OtherActor :type Actor%20Object%20Reference)))

(event EventTick
  (params (DeltaSeconds :type Float%20%28single-precision%29)))

(event EventBeginPlay)

(fn ConstructionScript)

(fn StartSprinting
  (Variables|/Script/Engine.CharacterMovementComponent|SetMaxWalkSpeed (Variables|Character|GetCharacterMovement) 7e+02))

(fn StopSprinting
  (Variables|/Script/Engine.CharacterMovementComponent|SetMaxWalkSpeed (Variables|Character|GetCharacterMovement) 3e+02))